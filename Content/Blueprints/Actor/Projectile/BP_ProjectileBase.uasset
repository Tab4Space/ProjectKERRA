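; Base projectile Blueprint that plays the sound and visual effects for a projectile's spawn, flight and impact.
; On BeginPlay it plays a spawn sound, attaches a flying sound that stops with the actor, and spawns a muzzle effect facing forward.
; OnSpawnProjectileHitFX plays impact sound and VFX at the given hit location.
; Each effect is skipped when its asset is unset, and this graph contains no movement or damage logic.
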(event `self.ReceiveBeginPlay`
  (`|ExecutionSequence`
    (:`then_0`
      (bind _projectilespawnsfx (`self.ProjectileSpawnSFX`)
        (:`then`
          (`GameplayStatics.PlaySoundAtLocation` _projectilespawnsfx (`self.K2_GetActorLocation`) (struct) 1.0 1.0 0.0 null null null null))
        (:`else`)))
    (:`then_1`
      (bind _projectileflyingsfx (`self.ProjectileFlyingSFX`)
        (:`then`
          (`GameplayStatics.SpawnSoundAttached` _projectileflyingsfx (`self.RootComponent`) "None" (0.0 0.0 0.0) (struct) "KeepRelativeOffset" true 1.0 1.0 0.0 null null))
        (:`else`)))
    (:`then_2`
      (bind _projectilemuzzlevfx (`self.ProjectileMuzzleVFX`)
        (:`then`
          (`NiagaraFunctionLibrary.SpawnSystemAtLocation` _projectilemuzzlevfx (`self.K2_GetActorLocation`) (`KismetMathLibrary.Conv_VectorToRotator` (`self.GetActorForwardVector`))))
        (:`else`)))))

(event `self.BP_OnSpawnProjectileHitFX`
  (params (HitLocation :type "Vector Structure (by ref)"))
  (`|ExecutionSequence`
    (:`then_0`
      (bind _projectileimpactsfx (`self.ProjectileImpactSFX`)
        (:`then`
          (`GameplayStatics.PlaySoundAtLocation` _projectileimpactsfx HitLocation (struct) 1.0 1.0 0.0 null null null null))
        (:`else`)))
    (:`then_1`
      (bind _projectileimpactvfx (`self.ProjectileImpactVFX`)
        (:`then`
          (`NiagaraFunctionLibrary.SpawnSystemAtLocation` _projectileimpactvfx HitLocation))
        (:`else`)))))

(fn `UserConstructionScript`)