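; BP_CameraManager is a player camera manager that provides a third-person, over-the-shoulder view of BP_KerraHero.
; It overrides BlueprintUpdateCamera to place the camera behind, right of and above the hero, using fixed offsets oriented by player 0's control rotation.
; The camera takes that control rotation and a fixed FOV directly, with no smoothing or collision check.
; The override only applies when the view target casts to BP_KerraHero.
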(fn `BlueprintUpdateCamera`
  (params (CameraTarget :type "Actor Object Reference"))
  (returns (NewCameraLocation :type "Vector Structure") (NewCameraRotation :type "Rotator Structure") (NewCameraFOV :type "Float (single-precision)") (ReturnValue :type Boolean))
  (bind _returnvalue (`Controller.GetControlRotation` (`GameplayStatics.GetPlayerController` 0)))
  (bind _asbp_kerra_hero (cast `/Game/Blueprints/Characters/Player/BP_KerraHero` CameraTarget))
  (return (+ (`self.K2_GetActorLocation` _asbp_kerra_hero) (+ (* (`KismetMathLibrary.GetForwardVector` _returnvalue) -350.0) (* (`KismetMathLibrary.GetRightVector` _returnvalue) 45.0)) (0.0 0.0 60.0)) (`Controller.GetControlRotation` (`GameplayStatics.GetPlayerController` 0)) 90.0 true))

(fn `UserConstructionScript`)