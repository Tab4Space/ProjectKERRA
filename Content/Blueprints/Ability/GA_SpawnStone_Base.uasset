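; Base Gameplay Ability that has a level-scaled chance to spawn a healing or rage stone near the avatar.
; On activation it traces down to the ground, then picks a random navigable point around the hit.
; It chooses either stone class at even odds, rolls the spawn chance from a scalable float at the ability level, then async loads the class before spawning it and ending.
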(event `self.K2_ActivateAbility`
  (bind _returnvalue (`self.GetAvatarActorFromActorInfo`))
  (bind _returnvalue_2 (`Actor.K2_GetActorLocation` _returnvalue))
  (`|ExecutionSequence`
    (:`then_0`
      (bind _outhit (`KismetSystemLibrary.LineTraceSingleForObjects` _returnvalue_2 (+ _returnvalue_2 (* (`Actor.GetActorUpVector` _returnvalue) -200.0)) (`self.Object Types`)))
      (bind _randomlocation (`NavigationSystemV1.K2_GetRandomLocationInNavigableRadius` (`.ImpactPoint` (`GameplayStatics.BreakHitResult` _outhit)) 200.0 null null))
      (set `self.RandomSpawnLocation` _randomlocation))
    (:`then_1`
      (if (`KismetMathLibrary.RandomBoolWithWeight` 0.5)
        (set `self.StoneClassToSpawn` "/Game/Blueprints/Actor/Item/PickUps/Stones/BP_HealingStone.BP_HealingStone_C")
        (else
          (set `self.StoneClassToSpawn` "/Game/Blueprints/Actor/Item/PickUps/Stones/BP_RageStone.BP_RageStone_C")))
      (if (`KismetMathLibrary.RandomBoolWithWeight` (`KerraFunctionLibrary.GetScalableFloatValueAtLevel` (`self.StoneSpawnChance`) (`KismetMathLibrary.Conv_IntToDouble` (`self.GetAbilityLevel`))))
        (bind _class (`|LoadAssetClass` (`self.StoneClassToSpawn`))
          (:`Completed`
            (bind _asactor (castclass `Actor` _class))
            (`|SpawnActorFromClass` _asactor (`KismetMathLibrary.MakeTransform` (`self.RandomSpawnLocation`)) "AdjustIfPossibleButAlwaysSpawn" "MultiplyWithRoot" null null)
            (`self.K2_EndAbility`)))
        (else
          (`self.K2_EndAbility`))))))