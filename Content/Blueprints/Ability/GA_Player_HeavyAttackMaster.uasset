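; Gameplay ability for the player's heavy attack combo, acting as a master that picks a montage from a map keyed by combo count.
; On activation it clears the reset timer, plays the current montage, and advances the count, wrapping after the last entry.
; When the montage completes, blends out, or is interrupted or cancelled, the ability ends and starts a short timer that resets the combo to the first attack.
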(event `self.K2_ActivateAbility`
  (`KismetSystemLibrary.K2_ClearAndInvalidateTimerHandle` (`self.ComboCountResetTimerHandle`))
  (`AbilityTask_PlayMontageAndWait.CreatePlayMontageAndWaitProxy` "None" (`BlueprintMapLibrary.Map_Find` (`self.AttackMontageMap`) (`self.CurrentHeavyAttackComboCount`))
    (:`then`
      (`|ExecutionSequence`
        (:`then_0`
          (if (== (`self.CurrentHeavyAttackComboCount`) (`BlueprintMapLibrary.Map_Length` (`self.AttackMontageMap`)))
            (`self.ResetAttackComboCount`)
            (else
              (`/Engine/EditorBlueprintResources/StandardMacros.IncrementInt` (`self.CurrentHeavyAttackComboCount`)))))))
    (:`OnCompleted`
      (`self.K2_EndAbility` :!label _label)
      (bind _returnvalue (`KismetSystemLibrary.K2_SetTimerDelegate` (delegate `ResetAttackComboCount`) 0.5))
      (set `self.ComboCountResetTimerHandle` _returnvalue))
    (:`OnBlendOut`
      (goto _label))
    (:`OnInterrupted`
      (goto _label))
    (:`OnCancelled`
      (goto _label))))

(event `ResetAttackComboCount`
  (set `self.CurrentHeavyAttackComboCount` 1))