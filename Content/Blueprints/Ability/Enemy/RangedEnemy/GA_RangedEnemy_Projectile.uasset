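; Gameplay ability that lets a ranged enemy fire a projectile during an attack montage.
; On activation it plays the montage and waits for the Shared.Event.SpawnProjectile gameplay event.
; That event spawns BP_RangedEnemy_Projectile at the mesh's Projectile socket, facing the enemy's forward vector and carrying a GE_DealDamage spec built from ProjectileDamage.
; The ability ends when the montage completes, blends out, is interrupted or is cancelled.
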(event `self.K2_ActivateAbility`
  (bind _returnvalue (`self.GetEnemyActorInfo`))
  (`AbilityTask_PlayMontageAndWait.CreatePlayMontageAndWaitProxy` "None" (`self.Montage to Play`)
    (:`then`
      (`AbilityTask_WaitGameplayEvent.WaitGameplayEvent` (struct :`TagName` "Shared.Event.SpawnProjectile") null
        (:`EventReceived`
          (`|SpawnActorFromClass` "/Game/Blueprints/Actor/Projectile/BP_RangedEnemy_Projectile.BP_RangedEnemy_Projectile_C" (`KismetMathLibrary.MakeTransform` (`SceneComponent.GetSocketLocation` (`self.GetOwningComponentFromActorInfo`) "Projectile") (`KismetMathLibrary.Conv_VectorToRotator` (`Actor.GetActorForwardVector` (`self.GetEnemyActorInfo`)))) "AdjustIfPossibleButAlwaysSpawn" "MultiplyWithRoot" _returnvalue (`self.MakeDamageEffectSpecHandle` "/Game/Blueprints/GameplayEffect/GE_DealDamage.GE_DealDamage_C" (`self.ProjectileDamage`)) _returnvalue))))
    (:`OnCompleted`
      (`self.K2_EndAbility` :!label _label))
    (:`OnBlendOut`
      (goto _label))
    (:`OnInterrupted`
      (goto _label))
    (:`OnCancelled`
      (goto _label))))