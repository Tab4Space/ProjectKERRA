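; Base gameplay ability that lets an enemy summon other enemies around itself.
; It plays a montage alongside a WaitSpawnEnemies task that uses the summon event tag to spawn a configurable class and count within a random radius of the caster.
; When spawning finishes it sets the HasSpawnedEnemies blackboard flag, and any montage completion, blend out, interruption or cancellation ends the ability.
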(event `self.K2_ActivateAbility`
  (`AbilityTask_PlayMontageAndWait.CreatePlayMontageAndWaitProxy` "None" (`self.Montage to Play`)
    (:`then`
      (`WaitSpawnEnemies.WaitSpawnEnemies` (struct :`TagName` "Enemy.Event.SummonEnemies") (`self.Soft Enemy Class to Spawn`) (`self.Num to Spawn`) (`Actor.K2_GetActorLocation` (`self.GetEnemyActorInfo`)) (`self.Random Spawn Radius`)
        (:`OnSpawnFinished`
          (`BlackboardComponent.SetValueAsBool` (`AIBlueprintHelperLibrary.GetBlackboard` (`self.GetEnemyActorInfo`)) "HasSpawnedEnemies" true))))
    (:`OnCompleted`
      (`self.K2_EndAbility` :!label _label))
    (:`OnBlendOut`
      (goto _label))
    (:`OnInterrupted`
      (goto _label))
    (:`OnCancelled`
      (goto _label))))