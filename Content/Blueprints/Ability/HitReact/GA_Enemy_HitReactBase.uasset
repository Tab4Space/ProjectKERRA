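; Base Gameplay Ability for enemy hit reactions, activated from a gameplay event.
; It optionally rotates the enemy to face the event instigator, then plays a random hit react montage, or waits briefly if none exist, before ending.
; A hit overlay material flashes on the mesh until the ability ends, and an under-attack Gameplay Effect is applied to the owner.
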(event `self.K2_ActivateAbilityFromEvent`
  (params (EventData :type "GameplayEventData Structure (by ref)"))
  (`|ExecutionSequence`
    (:`then_0`
      (if (`self.FaceAttacker`)
        (`Actor.K2_SetActorRotation` (`self.GetEnemyActorInfo`) (`KismetMathLibrary.FindLookAtRotation` (`Actor.K2_GetActorLocation` (`self.GetEnemyActorInfo`)) (`Actor.K2_GetActorLocation` (`.Instigator` (break `GameplayEventData` EventData)))) false)))
    (:`then_1`
      (if (`self.HasHitReactMontagesToPlay`)
        (`AbilityTask_PlayMontageAndWait.CreatePlayMontageAndWaitProxy` "None" (`KismetArrayLibrary.Array_Random` (`self.MontagesToPlay`))
          (:`then`
            (`MeshComponent.SetOverlayMaterial` (`self.GetOwningComponentFromActorInfo`) "/Game/Assets/Material/MI_HitOverlay.MI_HitOverlay"))
          (:`OnCompleted`
            (`self.K2_EndAbility` :!label _label))
          (:`OnBlendOut`
            (goto _label))
          (:`OnInterrupted`
            (goto _label))
          (:`OnCancelled`
            (goto _label)))
        (else
          (`MeshComponent.SetOverlayMaterial` (`self.GetOwningComponentFromActorInfo`) "/Game/Assets/Material/MI_HitOverlay.MI_HitOverlay")
          (if (not (`self.HasHitReactMontagesToPlay`))
            (`KismetSystemLibrary.Delay` 0.2)
            (`self.K2_EndAbility`)))))
    (:`then_2`
      (`self.K2_ApplyGameplayEffectSpecToOwner` (`self.MakeOutgoingGameplayEffectSpec` "/Game/Blueprints/Ability/GE_Enemy_UnderAttack.GE_Enemy_UnderAttack_C")))))

(event `self.K2_OnEndAbility`
  (params (bWasCancelled :type Boolean))
  (`MeshComponent.SetOverlayMaterial` (`self.GetOwningComponentFromActorInfo`) null))