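; Gameplay ability that sheathes the player's sword by playing an unequip montage.
; When the montage starts, it clears the equipped weapon tag, then waits for the unequip gameplay event to attach the sword to the pelvis socket.
; HandleUnequipWeapon then unlinks the weapon's anim layers, removes its input mapping context and revokes its granted abilities.
; The ability ends when the montage completes, blends out or is interrupted or cancelled.
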(event `self.K2_ActivateAbility`
  (`AbilityTask_PlayMontageAndWait.CreatePlayMontageAndWaitProxy` "None" "/Game/Blueprints/Characters/Player/Animations/Montage/AM_Unequip.AM_Unequip"
    (:`then`
      (set `KerraCombatComponent.CurrentEquippedWeaponTag` (struct) (`self.GetKerraCombatComponentFromActorInfo`))
      (`AbilityTask_WaitGameplayEvent.WaitGameplayEvent` (struct :`TagName` "Player.Event.Unequip.Sword") null
        (:`EventReceived`
          (`Actor.K2_AttachToComponent` (`KerraCombatComponent.GetCharacterCarriedWeaponByTag` (`self.GetKerraCombatComponentFromActorInfo`) (struct :`TagName` "Player.Weapon.Sword")) (`self.GetOwningComponentFromActorInfo`) "Weapon_Pelvis" "SnapToTarget" "KeepRelative" "KeepWorld" true)
          (`self.HandleUnequipWeapon` (cast `PlayerWeapon` (`KerraCombatComponent.GetCharacterCarriedWeaponByTag` (`self.GetKerraCombatComponentFromActorInfo`) (struct :`TagName` "Player.Weapon.Sword")) :!pure true)))))
    (:`OnCompleted`
      (`self.K2_EndAbility` :!label _label))
    (:`OnBlendOut`
      (goto _label))
    (:`OnInterrupted`
      (goto _label))
    (:`OnCancelled`
      (goto _label))))

(fn `HandleUnequipWeapon`
  (params (InWeaponToUnequip :type "PlayerWeapon Object Reference"))
  (locals (CachedWeaponData :type "KerraPlayerWeaponData Structure"))
  (bind (_weaponanimlayertolink _weaponinputmappingcontext) (break `KerraPlayerWeaponData` (`local.CachedWeaponData`)))
  (set `local.CachedWeaponData` (`PlayerWeapon.KerraPlayerWeaponData` InWeaponToUnequip))
  (`|ExecutionSequence`
    (:`then_0`
      (`SkeletalMeshComponent.UnlinkAnimClassLayers` (`self.GetOwningComponentFromActorInfo`) _weaponanimlayertolink))
    (:`then_1`
      (`EnhancedInputSubsystemInterface.RemoveMappingContext` (pcsubsystem `EnhancedInputLocalPlayerSubsystem` (`self.GetKerraPlayerControllerFromActorInfo`)) _weaponinputmappingcontext (struct)))
    (:`then_2`
      (`KerraAbilitySystemComponent.RemoveGrantedWeaponAbilities` (`self.GetKerraAbilitySystemComponentFromActorInfo`) (`PlayerWeapon.GetGrantedAbilitySpecHandles` (`local.InWeaponToUnequip`))))))