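; Gameplay ability that puts the Kerra player into Rage, playing an activation montage under a temporary Activating tag.
; A montage gameplay event adds the Rage cue, removed when the ability ends.
; The Rage cost effect is applied on activation and held by handle until the ability ends.
; The ability outlives the montage, cancelling itself when the Rage.None tag is added.
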(event `self.K2_ActivateAbility`
  (`KerraFunctionLibrary.AddGameplayTagToActorIfNone` (`self.GetKerraPlayerFromActorInfo`) (struct :`TagName` "Player.Status.Rage.Activating"))
  (`AbilityTask_PlayMontageAndWait.CreatePlayMontageAndWaitProxy` "None" "/Game/Blueprints/Characters/Player/Animations/Montage/AM_Activate_Rage.AM_Activate_Rage"
    (:`then`
      (`|ExecutionSequence`
        (:`then_0`
          (`AbilityTask_WaitGameplayEvent.WaitGameplayEvent` (struct :`TagName` "Player.Event.ActivateRage") null
            (:`EventReceived`
              (`self.K2_AddGameplayCueWithParams` (struct :`TagName` "GameplayCue.FX.Rage.Activating") (`AbilitySystemBlueprintLibrary.MakeGameplayCueParameters` 0.0 0.0 (struct) (struct) (struct) (struct) (struct) (0.0 0.0 0.0) (0.0 0.0 0.0) null null null null 1 1 (`self.GetOwningComponentFromActorInfo`))))))
        (:`then_1`
          (`AbilityTask_WaitGameplayTagAdded.WaitGameplayTagAdd` (struct :`TagName` "Player.Status.Rage.None") null
            (:`Added`
              (`self.K2_CancelAbility`))))
        (:`then_2`
          (bind _returnvalue (`self.BP_ApplyGameplayEffectToOwner` "/Game/Blueprints/Characters/Player/GameplayEffect/GE_Cost_Rage.GE_Cost_Rage_C" (`self.GetAbilityLevel`)))
          (set `self.ApplyCostRageGEHandle` _returnvalue))))
    (:`OnCompleted`
      (`KerraFunctionLibrary.RemoveGameplayTagFromActorIfFound` (`self.GetKerraPlayerFromActorInfo`) (struct :`TagName` "Player.Status.Rage.Activating") :!label _label))
    (:`OnBlendOut`
      (goto _label))
    (:`OnInterrupted`
      (goto _label))
    (:`OnCancelled`
      (goto _label))))

(event `self.K2_OnEndAbility`
  (params (bWasCancelled :type Boolean))
  (`self.BP_RemoveGameplayEffectFromOwnerWithHandle` (`self.ApplyCostRageGEHandle`)))