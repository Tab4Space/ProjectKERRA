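; Player light attack ability that plays a combo montage chosen by the current combo count.
; Each activation advances the count, resets it after a short post-montage timer unless reactivated, and wraps after the last attack.
; Melee hit events apply weapon damage scaled by combo count, play a hit sound cue and send hit reacts.
; The JumpToFinisher tag is added as the count reaches the final attack and removed on reset.
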(event `self.K2_ActivateAbility`
  (`KismetSystemLibrary.K2_ClearAndInvalidateTimerHandle` (`self.ComboCountResetTimerHandle`))
  (set `self.UsedComboCount` (`self.CurrentLightAttackComboCount`))
  (`AbilityTask_PlayMontageAndWait.CreatePlayMontageAndWaitProxy` "None" (`BlueprintMapLibrary.Map_Find` (`self.AttackMontageMap`) (`self.CurrentLightAttackComboCount`))
    (:`then`
      (`|ExecutionSequence`
        (:`then_0`
          (bind (_asynctaskproxy _payload) (`AbilityTask_WaitGameplayEvent.WaitGameplayEvent` (struct :`TagName` "Shared.Event.MeleeHit") null)
            (:`EventReceived`
              (`self.HandleApplyDamage` _payload))))
        (:`then_1`
          (if (== (`self.CurrentLightAttackComboCount`) (`BlueprintMapLibrary.Map_Length` (`self.AttackMontageMap`)))
            (`self.ResetAttackComboCount`)
            (else
              (if (== (`self.CurrentLightAttackComboCount`) (- (`BlueprintMapLibrary.Map_Length` (`self.AttackMontageMap`)) 1))
                (`KerraFunctionLibrary.AddGameplayTagToActorIfNone` (`self.GetKerraPlayerFromActorInfo`) (struct :`TagName` "Player.Status.JumpToFinisher")))
              (`/Engine/EditorBlueprintResources/StandardMacros.IncrementInt` (`self.CurrentLightAttackComboCount`)))))))
    (:`OnCompleted`
      (`self.K2_EndAbility` :!label _label)
      (bind _returnvalue (`KismetSystemLibrary.K2_SetTimerDelegate` (delegate `ResetAttackComboCount`) 0.5))
      (set `self.ComboCountResetTimerHandle` _returnvalue))
    (:`OnBlendOut`
      (goto _label))
    (:`OnInterrupted`
      (goto _label))
    (:`OnCancelled`
      (goto _label))))

(event `ResetAttackComboCount`
  (set `self.CurrentLightAttackComboCount` 1)
  (`KerraFunctionLibrary.RemoveGameplayTagFromActorIfFound` (`self.GetKerraPlayerFromActorInfo`) (struct :`TagName` "Player.Status.JumpToFinisher")))

(fn `HandleApplyDamage`
  (params (GameplayEventData :type "GameplayEventData Structure (by ref)"))
  (locals (LocalTargetActor :type "Actor Object Reference"))
  (set `local.LocalTargetActor` (`.Target` (break `GameplayEventData` GameplayEventData)))
  (`self.K2_ExecuteGameplayCue` (`self.WeaponHitSoundGCTag`))
  (`self.BP_ApplyEffectSpecHandleToTarget` (`local.LocalTargetActor`) (`self.MakePlayerDamageEffectSpecHandle` "/Game/Blueprints/Ability/GE_DealDamage.GE_DealDamage_C" (`HeroCombatComponent.GetPlayerCurrentEquippedWeaponDamageAtLevel` (`self.GetKerraPlayerCombatComponentFromActorInfo`) (`self.GetAbilityLevel`)) (struct :`TagName` "Player.SetByCaller.AttackType.Light") (`self.UsedComboCount`))
    (:`Successful`
      (`AbilitySystemBlueprintLibrary.SendGameplayEventToActor` (`local.LocalTargetActor`) (struct :`TagName` "Shared.Event.HitReact") (`local.GameplayEventData`)))))