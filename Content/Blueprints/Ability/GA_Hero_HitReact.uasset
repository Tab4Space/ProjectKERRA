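; Gameplay ability that plays the hero's directional hit reaction when activated by a gameplay event.
; It computes a front, left, right or back tag from the event's instigator and the player, then switches on it to pick the matching montage.
; A hit overlay material is applied while the montage plays.
; The ability ends when the montage completes, blends out, is interrupted or is cancelled, and ending clears the overlay.
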(event `self.K2_ActivateAbilityFromEvent`
  (params (EventData :type "GameplayEventData Structure (by ref)"))
  (`|SwitchGameplayTag` (`.ReturnValue` (`KerraFunctionLibrary.ComputeHitReactDirectionTag` (`.Instigator` (break `GameplayEventData` EventData)) (`self.GetKerraPlayerFromActorInfo`)))
    (:`Shared.Status.HitReact.Front`
      (set `self.Montage to Play` "/Game/Blueprints/Characters/Player/Animations/Montage/AM_Hero_HitReact_Front.AM_Hero_HitReact_Front"))
    (:`Shared.Status.HitReact.Left`
      (set `self.Montage to Play` "/Game/Blueprints/Characters/Player/Animations/Montage/AM_Hero_HitReact_Left.AM_Hero_HitReact_Left"))
    (:`Shared.Status.HitReact.Right`
      (set `self.Montage to Play` "/Game/Blueprints/Characters/Player/Animations/Montage/AM_Hero_HitReact_Right.AM_Hero_HitReact_Right"))
    (:`Shared.Status.HitReact.Back`
      (set `self.Montage to Play` "/Game/Blueprints/Characters/Player/Animations/Montage/AM_Hero_HitReact_Back.AM_Hero_HitReact_Back")))
  (`AbilityTask_PlayMontageAndWait.CreatePlayMontageAndWaitProxy` "None" (`self.Montage to Play`)
    (:`then`
      (`MeshComponent.SetOverlayMaterial` (`self.GetOwningComponentFromActorInfo`) "/Game/Assets/Material/MI_HitOverlay1.MI_HitOverlay1"))
    (:`OnCompleted`
      (`self.K2_EndAbility` :!label _label))
    (:`OnBlendOut`
      (goto _label))
    (:`OnInterrupted`
      (goto _label))
    (:`OnCancelled`
      (goto _label))))

(event `self.K2_OnEndAbility`
  (params (bWasCancelled :type Boolean))
  (`MeshComponent.SetOverlayMaterial` (`self.GetOwningComponentFromActorInfo`) null))