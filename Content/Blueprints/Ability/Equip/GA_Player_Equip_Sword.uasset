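; Gameplay ability that equips the player's sword, playing an equip montage and waiting for the sword equip gameplay event.
; On that event it snaps the carried sword to the right-hand weapon socket and records it as the equipped weapon tag.
; HandleEquipWeapon uses the weapon's data to link anim layers, add its input mapping context and grant abilities, storing their handles on the weapon.
; The ability ends when the montage finishes or is interrupted.
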(event `self.K2_ActivateAbility`
  (`AbilityTask_PlayMontageAndWait.CreatePlayMontageAndWaitProxy` "None" "/Game/Blueprints/Characters/Player/Animations/Montage/AM_Equip.AM_Equip"
    (:`then`
      (`AbilityTask_WaitGameplayEvent.WaitGameplayEvent` (struct :`TagName` "Player.Event.Equip.Sword") null
        (:`EventReceived`
          (`KismetSystemLibrary.PrintString` "Event Received")
          (`Actor.K2_AttachToComponent` (`KerraCombatComponent.GetCharacterCarriedWeaponByTag` (`self.GetKerraPlayerCombatComponentFromActorInfo`) (struct :`TagName` "Player.Weapon.Sword")) (`self.GetOwningComponentFromActorInfo`) "Weapon_R" "SnapToTarget" "KeepRelative" "KeepWorld" true)
          (`self.HandleEquipWeapon` (`KerraPlayerCombatComponent.GetPlayerCarriedWeaponByTag` (`self.GetKerraPlayerCombatComponentFromActorInfo`) (struct :`TagName` "Player.Weapon.Sword")))
          (set `KerraCombatComponent.CurrentEquippedWeaponTag` (struct :`TagName` "Player.Weapon.Sword") (`self.GetKerraPlayerCombatComponentFromActorInfo`)))))
    (:`OnCompleted`
      (`self.K2_EndAbility` :!label _label))
    (:`OnBlendOut`
      (goto _label))
    (:`OnInterrupted`
      (goto _label))
    (:`OnCancelled`
      (goto _label))))

(fn `HandleEquipWeapon`
  (params (InWeaponToEquip :type "PlayerWeapon Object Reference"))
  (locals (CachedWeaponData :type "KerraPlayerWeaponData Structure"))
  (bind (_weaponanimlayertolink _weaponinputmappingcontext _defaultweaponabilities) (break `KerraPlayerWeaponData` (`local.CachedWeaponData`)))
  (set `local.CachedWeaponData` (`PlayerWeapon.KerraPlayerWeaponData` InWeaponToEquip))
  (`|ExecutionSequence`
    (:`then_0`
      (`SkeletalMeshComponent.LinkAnimClassLayers` (`self.GetOwningComponentFromActorInfo`) _weaponanimlayertolink))
    (:`then_1`
      (`EnhancedInputSubsystemInterface.AddMappingContext` (pcsubsystem `EnhancedInputLocalPlayerSubsystem` (`self.GetKerraPlayerControllerFromActorInfo`)) _weaponinputmappingcontext 1 (struct)))
    (:`then_2`
      (bind _outgrantedabilityspechandles (`KerraAbilitySystemComponent.GrantWeaponAbilities` (`self.GetKerraAbilitySystemComponentFromActorInfo`) _defaultweaponabilities (`self.GetAbilityLevel`)))
      (`PlayerWeapon.AssignGrantedAbilitySpecHandles` (`local.InWeaponToEquip`) _outgrantedabilityspechandles))))