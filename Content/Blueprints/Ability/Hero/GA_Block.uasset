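; Player block ability that plays a block montage with a magic shield gameplay cue while active.
; A successful-block event turns the player toward the attacker, applies backward root-motion knockback and fires an impact cue.
; Blocks landing shortly after activation count as perfect, adding a perfect-block cue, brief global slow motion and a short-lived JumpToFinisher tag.
; Ending the ability restores normal time dilation.
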(event `self.K2_ActivateAbility`
  (set `self.BlockActivateTime` (`GameplayStatics.GetTimeSeconds`))
  (`AbilityTask_PlayMontageAndWait.CreatePlayMontageAndWaitProxy` "None" "/Game/Blueprints/Characters/Player/Animations/Montages/AM_Block.AM_Block"
    (:`then`
      (`|ExecutionSequence`
        (:`then_0`
          (`self.K2_AddGameplayCueWithParams` (struct :`TagName` "GameplayCue.FX.MagicShield") (`self.MakeBlockGCParams`)))
        (:`then_1`
          (bind (_asynctaskproxy _payload) (`AbilityTask_WaitGameplayEvent.WaitGameplayEvent` (struct :`TagName` "Player.Event.SuccessBlock") null)
            (:`EventReceived`
              (set `self.IsPerfectBlock` (<= (- (`GameplayStatics.GetTimeSeconds`) (`self.BlockActivateTime`)) 0.25))
              (`|ExecutionSequence`
                (:`then_0`
                  (`Actor.K2_SetActorRotation` (`self.GetKerraPlayerFromActorInfo`) (`KismetMathLibrary.FindLookAtRotation` (`Actor.K2_GetActorLocation` (`self.GetKerraPlayerFromActorInfo`)) (`Actor.K2_GetActorLocation` (`.Instigator` (break `GameplayEventData` _payload)))) false))
                (:`then_1`
                  (`AbilityTask_ApplyRootMotionConstantForce.ApplyRootMotionConstantForce` "None" (* (`Actor.GetActorForwardVector` (`self.GetKerraPlayerFromActorInfo`)) -1.0) 300.0 0.2 false null "MaintainLastRootMotionVelocity"))
                (:`then_2`
                  (`self.K2_ExecuteGameplayCueWithParams` (struct :`TagName` "GameplayCue.FX.MagicShield.SuccessfulBlock") (`self.MakeBlockGCParams`)))
                (:`then_3`
                  (if (`self.IsPerfectBlock`)
                    (`KerraFunctionLibrary.AddGameplayTagToActorIfNone` (`self.GetKerraPlayerFromActorInfo`) (struct :`TagName` "Player.Status.JumpToFinisher"))
                    (`self.K2_ExecuteGameplayCueWithParams` (struct :`TagName` "GameplayCue.FX.MagicShield.PerfectBlock") (`self.MakeBlockGCParams`))
                    (`GameplayStatics.SetGlobalTimeDilation` 0.2)
                    (`KismetSystemLibrary.Delay` 0.08)
                    (`GameplayStatics.SetGlobalTimeDilation` 1.0)
                    (`self.StartResetJumpToFinisherTimer`)))))))))
    (:`OnInterrupted`
      (`self.K2_EndAbility` :!label _label)
      (`self.StartResetJumpToFinisherTimer`))
    (:`OnCancelled`
      (goto _label))))

(event `self.K2_OnEndAbility`
  (params (bWasCancelled :type Boolean))
  (if (!= (`GameplayStatics.GetGlobalTimeDilation`) 1.0)
    (`GameplayStatics.SetGlobalTimeDilation` 1.0)))

(event `StartResetJumpToFinisherTimer`
  (`KismetSystemLibrary.K2_SetTimerDelegate` (delegate `ResetJumpToFinisherState`) 0.3))

(event `ResetJumpToFinisherState`
  (`KerraFunctionLibrary.RemoveGameplayTagFromActorIfFound` (`self.GetKerraPlayerFromActorInfo`) (struct :`TagName` "Player.Status.JumpToFinisher")))

(fn `MakeBlockGCParams`
  (returns (ReturnValue :type "GameplayCueParameters Structure"))
  (return (`AbilitySystemBlueprintLibrary.MakeGameplayCueParameters` 0.0 0.0 (struct) (struct) (struct) (struct) (struct) (0.0 0.0 0.0) (0.0 0.0 0.0) null null null null 1 1 (`self.GetOwningComponentFromActorInfo`))))