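; Base Gameplay Ability for the hero's heavy melee combo, playing the montage for the current combo step or jumping to the finisher when the player has the JumpToFinisher tag.
; Each activation advances the count, which wraps after the last step or resets shortly after the montage ends.
; MeleeHit events apply combo-scaled weapon damage, sending hit reacts and granting rage on success.
; An active Rage tag triggers WhileRageActive, an empty hook here.
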(event `self.K2_ActivateAbility`
  (`KismetSystemLibrary.K2_ClearAndInvalidateTimerHandle` (`self.ComboCountResetTimerHandle`))
  (`KerraFunctionLibrary.BP_DoesActorHaveTag` (`self.GetKerraPlayerFromActorInfo`) (struct :`TagName` "Player.Status.JumpToFinisher")
    (:`Yes`
      (set `self.CurrentHeavyAttackComboCount` (`BlueprintMapLibrary.Map_Length` (`self.AttackMontageMap`))))
    (:`No`
      _))
  (set `self.UsedComboCound` (`self.CurrentHeavyAttackComboCount`))
  (`AbilityTask_PlayMontageAndWait.CreatePlayMontageAndWaitProxy` "None" (`BlueprintMapLibrary.Map_Find` (`self.AttackMontageMap`) (`self.CurrentHeavyAttackComboCount`))
    (:`then`
      (`|ExecutionSequence`
        (:`then_0`
          (bind (_asynctaskproxy _payload) (`AbilityTask_WaitGameplayEvent.WaitGameplayEvent` (struct :`TagName` "Shared.Event.MeleeHit") null)
            (:`EventReceived`
              (`self.HandleApplyDamage` _payload))))
        (:`then_1`
          (if (== (`self.CurrentHeavyAttackComboCount`) (`BlueprintMapLibrary.Map_Length` (`self.AttackMontageMap`)))
            (`self.ResetAttackComboCount`)
            (else
              (`/Engine/EditorBlueprintResources/StandardMacros.IncrementInt` (`self.CurrentHeavyAttackComboCount`)))))
        (:`then_2`
          (`KerraFunctionLibrary.BP_DoesActorHaveTag` (`self.GetKerraPlayerFromActorInfo`) (struct :`TagName` "Player.Status.Rage.Active")
            (:`Yes`
              (`self.WhileRageActive`))))))
    (:`OnCompleted`
      (`self.K2_EndAbility` :!label _label)
      (bind _returnvalue (`KismetSystemLibrary.K2_SetTimerDelegate` (delegate `ResetAttackComboCount`) 0.5))
      (set `self.ComboCountResetTimerHandle` _returnvalue))
    (:`OnBlendOut`
      (goto _label))
    (:`OnInterrupted`
      (goto _label))
    (:`OnCancelled`
      (goto _label))))

(event `WhileRageActive`)

(event `ResetAttackComboCount`
  (set `self.CurrentHeavyAttackComboCount` 1)
  (`KerraFunctionLibrary.RemoveGameplayTagFromActorIfFound` (`self.GetKerraPlayerFromActorInfo`) (struct :`TagName` "Player.Status.JumpToFinisher")))

(fn `HandleApplyDamage`
  (params (GameplayEventData :type "GameplayEventData Structure (by ref)"))
  (locals (LocalTargetActor :type "Actor Object Reference"))
  (set `local.LocalTargetActor` (`.Target` (break `GameplayEventData` GameplayEventData)))
  (`self.K2_ExecuteGameplayCue` (`self.WeaponHitSoundGCTag`))
  (`self.BP_ApplyEffectSpecHandleToTarget` (`local.LocalTargetActor`) (`self.MakeDamageEffectSpecHandle` "/Game/Blueprints/GameplayEffect/GE_DealDamage.GE_DealDamage_C" (`HeroCombatComponent.GetPlayerCurrentEquippedWeaponDamageAtLevel` (`self.GetKerraPlayerCombatComponentFromActorInfo`) (`self.GetAbilityLevel`)) (struct :`TagName` "Player.SetByCaller.AttackType.Heavy") (`self.UsedComboCound`))
    (:`Successful`
      (`AbilitySystemBlueprintLibrary.SendGameplayEventToActor` (`local.LocalTargetActor`) (struct :`TagName` "Shared.Event.HitReact") (`local.GameplayEventData`))
      (`self.BP_ApplyGameplayEffectToOwner` "/Game/Blueprints/Characters/Player/GameplayEffect/GE_GainRage.GE_GainRage_C" (`self.GetAbilityLevel`)))))