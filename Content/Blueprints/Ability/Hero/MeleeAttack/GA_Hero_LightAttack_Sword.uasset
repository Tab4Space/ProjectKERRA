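; Hero light sword attack ability that adds a slash projectile while rage is active, with activation and end events left to the parent.
; WhileRageActive waits for the SpawnProjectile gameplay event, then spawns BP_Slash at the equipped weapon's RageSlashSocket, yawed along the player's forward vector and rolled with the socket.
; The slash receives a damage effect spec built from weapon damage at ability level, tagged as a light attack with a fixed combo count.
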(event `self.WhileRageActive`
  (bind _returnvalue (`self.GetKerraPlayerFromActorInfo`))
  (bind (_returnvalue_roll _returnvalue_pitch _returnvalue_yaw) (`KismetMathLibrary.BreakRotator` (`KismetMathLibrary.MakeRotFromX` (`Actor.GetActorForwardVector` (`self.GetKerraPlayerFromActorInfo`)))))
  (bind _returnvalue_2 (`SceneComponent.GetSocketTransform` (`KerraWeaponBase.WeaponMesh` (`KerraCombatComponent.GetCharacterCurrentEquippedWeapon` (`self.GetKerraPlayerCombatComponentFromActorInfo`))) "RageSlashSocket" "RTS_World"))
  (`AbilityTask_WaitGameplayEvent.WaitGameplayEvent` (struct :`TagName` "Shared.Event.SpawnProjectile") null
    (:`EventReceived`
      (`|SpawnActorFromClass` "/Game/Blueprints/Actor/Projectile/BP_Slash.BP_Slash_C" (`KismetMathLibrary.MakeTransform` (.location _returnvalue_2) (`KismetMathLibrary.MakeRotator` (.roll (.rotation _returnvalue_2)) 0.0 _returnvalue_yaw)) "AdjustIfPossibleButAlwaysSpawn" "MultiplyWithRoot" _returnvalue (`self.MakeDamageEffectSpecHandle` "/Game/Blueprints/GameplayEffect/GE_DealDamage.GE_DealDamage_C" (`HeroCombatComponent.GetPlayerCurrentEquippedWeaponDamageAtLevel` (`self.GetKerraPlayerCombatComponentFromActorInfo`) (`self.GetAbilityLevel`)) (struct :`TagName` "Player.Ability.Attack.Light") 3) _returnvalue))))