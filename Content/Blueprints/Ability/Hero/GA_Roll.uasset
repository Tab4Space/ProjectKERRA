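; Gameplay ability that makes the hero perform a dodge roll in the last movement input direction, using root motion and motion warping.
; After a brief delay, it sets a facing warp target and traces down from a level-scaled roll distance to find the landing point.
; A ground hit sets the location warp target, while a miss removes it.
; It then plays the roll montage and ends when that completes, blends out or is interrupted.
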(event `self.K2_ActivateAbility`
  (`KismetSystemLibrary.Delay` 0.05)
  (`self.ComputeRollDirectionAndDistance`)
  (`AbilityTask_PlayMontageAndWait.CreatePlayMontageAndWaitProxy` "None" "/Game/Blueprints/Characters/Player/Animations/Montages/AM_Roll_RM.AM_Roll_RM"
    (:`OnCompleted`
      _)
    (:`OnBlendOut`
      _)
    (:`OnInterrupted`
      _)
    (:`OnCancelled`
      _))
  (`self.K2_EndAbility`))

(fn `ComputeRollDirectionAndDistance`
  (locals (CachedRollDirection :type "Vector Structure" :default (0.0 0.0 0.0)))
  (bind _returnvalue (`self.GetKerraPlayerFromActorInfo`))
  (bind _returnvalue_2 (+ (`Actor.K2_GetActorLocation` (`self.GetKerraPlayerFromActorInfo`)) (* (`local.CachedRollDirection`) (`KerraFunctionLibrary.GetScalableFloatValueAtLevel` (`self.RollingDistance`) (`KismetMathLibrary.Conv_IntToDouble` (`self.GetAbilityLevel`))))))
  (set `local.CachedRollDirection` (`KismetMathLibrary.Normal` (`Pawn.GetLastMovementInputVector` _returnvalue)))
  (`|ExecutionSequence`
    (:`then_0`
      (`MotionWarpingComponent.AddOrUpdateWarpTargetFromLocationAndRotation` (`KerraCharacterBase.MotionWarpingComponent` _returnvalue) "RollingDirection" (0.0 0.0 0.0) (`KismetMathLibrary.MakeRotFromX` (`local.CachedRollDirection`))))
    (:`then_1`
      (bind (_outhit _returnvalue_3) (`KismetSystemLibrary.LineTraceSingleForObjects` :`Start` _returnvalue_2 :`End` (+ _returnvalue_2 (* (* (`Actor.GetActorUpVector` (`self.GetKerraPlayerFromActorInfo`)) -1.0) 500.0)) :`ObjectTypes` (`self.Object Types`) :`DrawDebugType` "ForDuration"))
      (if _returnvalue_3
        (`MotionWarpingComponent.AddOrUpdateWarpTargetFromLocation` (`KerraCharacterBase.MotionWarpingComponent` (`self.GetKerraPlayerFromActorInfo`)) "RollTargetLocation" (`.ImpactPoint` (`GameplayStatics.BreakHitResult` _outhit)))
        (else
          (`MotionWarpingComponent.RemoveWarpTarget` (`KerraCharacterBase.MotionWarpingComponent` (`self.GetKerraPlayerFromActorInfo`)) "RollTargetLocation"))))))