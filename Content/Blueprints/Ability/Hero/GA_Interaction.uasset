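; GA_Interaction is a gameplay ability that lets the avatar interact with quest NPCs and collectable items in front of it.
; On activation it runs a short forward sphere trace with debug drawing and checks the hit actor for KerraQuestInterface.
; It casts to BP_KerraNpc, then BP_CollectableItemBase, and calls DoInteraction with the avatar.
; The ability ends only after a successful interaction; unconnected quest component calls never run.
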(event `self.K2_ActivateAbility`
  (bind _returnvalue (`self.GetAvatarActorFromActorInfo`))
  (bind _returnvalue_2 (`Actor.K2_GetActorLocation` _returnvalue))
  (bind _outhit (`KismetSystemLibrary.SphereTraceSingleForObjects` _returnvalue_2 (+ _returnvalue_2 (* (`Actor.GetActorForwardVector` _returnvalue) 100.0)) 50.0 (`|MakeArray` "ObjectTypeQuery3" "ObjectTypeQuery2" :!type "EObjectTypeQuery Enum") false (`|MakeArray` _returnvalue) "ForDuration"))
  (bind (_bblockinghit _binitialoverlap _time _distance _location _impactpoint _normal _impactnormal _physmat _hitactor) (`GameplayStatics.BreakHitResult` _outhit))
  (if (`KismetSystemLibrary.DoesImplementInterface` _hitactor "/Script/Kerra.KerraQuestInterface")
    (bind _asbp_kerra_npc (cast `/Game/Blueprints/Characters/NPC/BP_KerraNpc` _hitactor)
      (:`then`
        (`KerraNpc.DoInteraction` _asbp_kerra_npc (`self.GetAvatarActorFromActorInfo`))
        (`self.K2_EndAbility`))
      (:`CastFailed`
        (bind _asbp_collectable_item_base (cast `/Game/Blueprints/Actor/Item/Colletable/BP_CollectableItemBase` _hitactor))
        (`KerraCollectableBase.DoInteraction` _asbp_collectable_item_base (`self.GetAvatarActorFromActorInfo`))
        (`self.K2_EndAbility`)))))