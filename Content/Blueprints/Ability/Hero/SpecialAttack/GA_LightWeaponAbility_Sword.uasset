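; Gameplay ability for the hero's light special sword attack, which plays a montage and damages targets it hits.
; On activation it listens for melee hit events while committing the ability and starting the UI cooldown, then ends when the montage finishes or is interrupted.
; Each hit applies a damage effect using equipped weapon damage at ability level, tagged as a heavy attack, then fires a hit sound cue and sends a hit-react event.
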(event `self.K2_ActivateAbility`
  (bind _returnvalue (`self.GetCooldownTimeRemaining`))
  (`AbilityTask_PlayMontageAndWait.CreatePlayMontageAndWaitProxy` "None" "/Game/Blueprints/Characters/Player/Animations/Montages/AM_SpecialWeaponAbility_Light_Long.AM_SpecialWeaponAbility_Light_Long"
    (:`then`
      (`|ExecutionSequence`
        (:`then_0`
          (bind (_asynctaskproxy _payload) (`AbilityTask_WaitGameplayEvent.WaitGameplayEvent` (struct :`TagName` "Shared.Event.MeleeHit") null)
            (:`EventReceived`
              (`self.HandleApplyDamage` _payload))))
        (:`then_1`
          (`self.K2_CommitAbility`)
          (`HeroUIComponent.OnAbilityCooldownBegin` (`KerraHero.UIComponent` (`self.GetKerraPlayerFromActorInfo`)) (struct :`TagName` "InputTag.SpecialWeaponAbility.Light") _returnvalue _returnvalue))))
    (:`OnCompleted`
      (`self.K2_EndAbility` :!label _label))
    (:`OnBlendOut`
      (goto _label))
    (:`OnInterrupted`
      (goto _label))
    (:`OnCancelled`
      (goto _label))))

(fn `HandleApplyDamage`
  (params (InPayload :type "GameplayEventData Structure (by ref)"))
  (locals (LocalTargetActor :type "Actor Object Reference"))
  (set `local.LocalTargetActor` (`.Target` (break `GameplayEventData` InPayload)))
  (`self.BP_ApplyEffectSpecHandleToTarget` (`local.LocalTargetActor`) (`self.MakeDamageEffectSpecHandle` "/Game/Blueprints/GameplayEffect/GE_DealDamage.GE_DealDamage_C" (`HeroCombatComponent.GetPlayerCurrentEquippedWeaponDamageAtLevel` (`self.GetKerraPlayerCombatComponentFromActorInfo`) (`self.GetAbilityLevel`)) (struct :`TagName` "Player.SetByCaller.AttackType.Heavy") 3)
    (:`Successful`
      (`self.K2_ExecuteGameplayCue` (`self.WeaponHitSoundGCTag`))
      (`AbilitySystemBlueprintLibrary.SendGameplayEventToActor` (`local.LocalTargetActor`) (struct :`TagName` "Shared.Event.HitReact") (`local.InPayload`)))))