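; Player gameplay ability that equips the carried sword, playing an equip montage and ending when it finishes or is interrupted.
; A montage gameplay event attaches the sword to the hand socket and records it as the equipped weapon.
; HandleEquipWeapon then applies the weapon's data: linked anim layers, input mapping context and granted abilities, storing spec handles on the weapon.
; It also refreshes the UI weapon icon, ability slots and any running cooldowns.
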(event `self.K2_ActivateAbility`
  (bind _charactermovement (`Character.CharacterMovement` (`self.GetKerraPlayerFromActorInfo`)))
  (set `CharacterMovementComponent.bOrientRotationToMovement` true _charactermovement)
  (set `CharacterMovementComponent.RotationRate` (`KismetMathLibrary.MakeRotator` 0.0 0.0 500.0) _charactermovement)
  (`AbilityTask_PlayMontageAndWait.CreatePlayMontageAndWaitProxy` "None" "/Game/Blueprints/Characters/Player/Animations/Montages/AM_Equip.AM_Equip"
    (:`then`
      (`AbilityTask_WaitGameplayEvent.WaitGameplayEvent` (struct :`TagName` "Player.Event.Equip.Sword") null
        (:`EventReceived`
          (`KismetSystemLibrary.PrintString` "Event Received")
          (`Actor.K2_AttachToComponent` (`KerraCombatComponent.GetCharacterCarriedWeaponByTag` (`self.GetKerraPlayerCombatComponentFromActorInfo`) (struct :`TagName` "Player.Weapon.Sword")) (`self.GetOwningComponentFromActorInfo`) "Weapon_R" "SnapToTarget" "KeepRelative" "KeepWorld" true)
          (`self.HandleEquipWeapon` (`HeroCombatComponent.GetPlayerCarriedWeaponByTag` (`self.GetKerraPlayerCombatComponentFromActorInfo`) (struct :`TagName` "Player.Weapon.Sword")))
          (set `KerraCombatComponent.CurrentEquippedWeaponTag` (struct :`TagName` "Player.Weapon.Sword") (`self.GetKerraPlayerCombatComponentFromActorInfo`)))))
    (:`OnCompleted`
      (`self.K2_EndAbility` :!label _label))
    (:`OnBlendOut`
      (goto _label))
    (:`OnInterrupted`
      (goto _label))
    (:`OnCancelled`
      (goto _label))))

(fn `HandleEquipWeapon`
  (params (InWeaponToEquip :type "HeroWeapon Object Reference"))
  (locals (CachedWeaponData :type "KerraPlayerWeaponData Structure"))
  (bind (_weaponanimlayertolink _weaponinputmappingcontext _defaultweaponabilities _specialweaponabilities _weaponbasedamage _softweaponicontexture) (break `KerraPlayerWeaponData` (`local.CachedWeaponData`)))
  (set `local.CachedWeaponData` (`HeroWeapon.KerraPlayerWeaponData` InWeaponToEquip))
  (`|ExecutionSequence`
    (:`then_0`
      (`SkeletalMeshComponent.LinkAnimClassLayers` (`self.GetOwningComponentFromActorInfo`) _weaponanimlayertolink))
    (:`then_1`
      (`EnhancedInputSubsystemInterface.AddMappingContext` (pcsubsystem `EnhancedInputLocalPlayerSubsystem` (`self.GetKerraPlayerControllerFromActorInfo`)) _weaponinputmappingcontext 1 (struct)))
    (:`then_2`
      (bind _outgrantedabilityspechandles (`KerraAbilitySystemComponent.GrantWeaponAbilities` (`self.GetKerraAbilitySystemComponentFromActorInfo`) _defaultweaponabilities _specialweaponabilities (`self.GetAbilityLevel`)))
      (`HeroWeapon.AssignGrantedAbilitySpecHandles` (`local.InWeaponToEquip`) _outgrantedabilityspechandles))
    (:`then_3`
      (`HeroUIComponent.OnEquippedWeaponChanged` (`KerraHero.UIComponent` (`self.GetKerraPlayerFromActorInfo`)) _softweaponicontexture)
      (for _array_element (`.SpecialWeaponAbilities` (break `KerraPlayerWeaponData` (`local.CachedWeaponData`)))
        (bind (_softabilityiconmaterial _abilitycooldowntag _inputtag) (break `KerraPlayerSpecialAbilitySet` _array_element))
        (`HeroUIComponent.OnAbilityIconSlotUpdated` (`KerraHero.UIComponent` (`self.GetKerraPlayerFromActorInfo`)) _inputtag _softabilityiconmaterial)
        (bind (_totalcooldowntime _remainingcooldowntime _returnvalue) (`self.GetAbilityRemainingCooldownByTag` _abilitycooldowntag))
        (if _returnvalue
          (`HeroUIComponent.OnAbilityCooldownBegin` (`KerraHero.UIComponent` (`self.GetKerraPlayerFromActorInfo`)) _inputtag _totalcooldowntime _remainingcooldowntime))))))