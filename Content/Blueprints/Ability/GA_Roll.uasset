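; GA_Roll is the Kerra player's roll gameplay ability, playing a root-motion roll montage.
; After a brief delay, it caches the normalized last movement input and sets it as the rotation of the "RollingDirection" motion warping target.
; It then plays the montage and ends on completion, blend out, interruption or cancellation.
; The downward trace that would set "RollTargetLocation" from a level-scaled RollingDistance is unconnected, so only direction is warped.
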(event `self.K2_ActivateAbility`
  (`KismetSystemLibrary.Delay` 0.05)
  (`self.ComputeRollDirectionAndDistance`)
  (`AbilityTask_PlayMontageAndWait.CreatePlayMontageAndWaitProxy` "None" "/Game/Blueprints/Characters/Player/Animations/Montage/AM_Roll_RM.AM_Roll_RM"
    (:`OnCompleted`
      _)
    (:`OnBlendOut`
      _)
    (:`OnInterrupted`
      _)
    (:`OnCancelled`
      _))
  (`self.K2_EndAbility`))

(fn `ComputeRollDirectionAndDistance`
  (locals (CachedRollDirection :type "Vector Structure" :default (0.0 0.0 0.0)))
  (bind _returnvalue (`self.GetKerraPlayerFromActorInfo`))
  (set `local.CachedRollDirection` (`KismetMathLibrary.Normal` (`Pawn.GetLastMovementInputVector` _returnvalue)))
  (`|ExecutionSequence`
    (:`then_0`
      (`MotionWarpingComponent.AddOrUpdateWarpTargetFromLocationAndRotation` (`KerraCharacterBase.MotionWarpingComponent` _returnvalue) "RollingDirection" (0.0 0.0 0.0) (`KismetMathLibrary.MakeRotFromX` (`local.CachedRollDirection`))))))