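; Base gameplay ability for enemy melee attacks, running an attack montage that deals damage on hit.
; Enemies tagged Unblockable first fire a warning gameplay cue and briefly delay.
; While the montage plays, a MeleeHit gameplay event triggers damage through an effect spec; successful application executes a cue and forwards a HitReact event to the target.
; The ability ends when the montage completes, blends out, or is interrupted or cancelled.
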(event `self.K2_ActivateAbility`
  (`KerraFunctionLibrary.BP_DoesActorHaveTag` (`self.GetEnemyActorInfo`) (struct :`TagName` "Enemy.Status.Unblockable")
    (:`Yes`
      (`self.K2_ExecuteGameplayCueWithParams` (struct :`TagName` "GameplayCue.FX.UnblockableWarning") (`AbilitySystemBlueprintLibrary.MakeGameplayCueParameters` 0.0 (`self.UnblockableWarningSpawnOffset`)))
      (`KismetSystemLibrary.Delay` 0.2))
    (:`No`
      _))
  (`AbilityTask_PlayMontageAndWait.CreatePlayMontageAndWaitProxy` "None" (`self.Montage to Play`)
    (:`then`
      (bind (_asynctaskproxy _payload) (`AbilityTask_WaitGameplayEvent.WaitGameplayEvent` (struct :`TagName` "Shared.Event.MeleeHit") null)
        (:`EventReceived`
          (`self.HandleApplyDamage` _payload))))
    (:`OnCompleted`
      (`self.K2_EndAbility` :!label _label))
    (:`OnBlendOut`
      (goto _label))
    (:`OnInterrupted`
      (goto _label))
    (:`OnCancelled`
      (goto _label))))

(fn `HandleApplyDamage`
  (params (InPayload :type "GameplayEventData Structure"))
  (bind (_eventtag _instigator _target) (break `GameplayEventData` InPayload))
  (`self.BP_ApplyEffectSpecHandleToTarget` _target (`self.MakeDamageEffectSpecHandle` "/Game/Blueprints/Ability/GE_DealDamage.GE_DealDamage_C" (`self.In Damage Float`))
    (:`Successful`
      (`|ExecutionSequence`
        (:`then_0`
          (`self.K2_ExecuteGameplayCue` (struct)))
        (:`then_1`
          (`AbilitySystemBlueprintLibrary.SendGameplayEventToActor` _target (struct :`TagName` "Shared.Event.HitReact") (`local.InPayload`)))))))