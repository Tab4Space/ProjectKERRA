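; GA_HeavyWeaponAbility_Sword is the Kerra player's sword heavy special weapon ability, an area attack driven by a montage.
; On activation it plays the montage, commits the ability and tells the player UI to begin the cooldown display.
; A gameplay event triggers a forward box trace, applying a heavy-attack damage spec scaled by equipped weapon damage to the hits.
; The ability ends when the montage completes, blends out or is stopped.
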(event `self.K2_ActivateAbility`
  (bind _returnvalue (`self.GetKerraPlayerFromActorInfo`))
  (bind _returnvalue_2 (`self.GetCooldownTimeRemaining`))
  (bind _returnvalue_3 (`Actor.K2_GetActorLocation` _returnvalue))
  (bind _returnvalue_4 (`Actor.GetActorForwardVector` _returnvalue))
  (`AbilityTask_PlayMontageAndWait.CreatePlayMontageAndWaitProxy` "None" "/Game/Blueprints/Characters/Player/Animations/Montage/AM_SpecialWeaponAbility_Heavy.AM_SpecialWeaponAbility_Heavy"
    (:`then`
      (`|ExecutionSequence`
        (:`then_0`
          (`self.K2_CommitAbility`)
          (`HeroUIComponent.OnAbilityCooldownBegin` (`KerraHero.UIComponent` (`self.GetKerraPlayerFromActorInfo`)) (struct :`TagName` "InputTag.SpecialWeaponAbility.Heavy") _returnvalue_2 _returnvalue_2))
        (:`then_1`
          (`AbilityTask_WaitGameplayEvent.WaitGameplayEvent` (struct :`TagName` "Player.Event.AOE") null
            (:`EventReceived`
              (bind _outhits (`KismetSystemLibrary.BoxTraceMultiForObjects` _returnvalue_3 (+ _returnvalue_3 (* _returnvalue_4 200.0)) (250.0 250.0 250.0) (`KismetMathLibrary.Conv_VectorToRotator` _returnvalue_4) (`self.Object Types`)))
              (`self.ApplyGameplaySpecHandleToHitResults` (`self.MakeDamageEffectSpecHandle` "/Game/Blueprints/Ability/GE_DealDamage.GE_DealDamage_C" (`HeroCombatComponent.GetPlayerCurrentEquippedWeaponDamageAtLevel` (`self.GetKerraPlayerCombatComponentFromActorInfo`) (`self.GetAbilityLevel`)) (struct :`TagName` "Player.SetByCaller.AttackType.Heavy") 3) _outhits))))))
    (:`OnCompleted`
      (`self.K2_EndAbility` :!label _label))
    (:`OnBlendOut`
      (goto _label))
    (:`OnInterrupted`
      (goto _label))
    (:`OnCancelled`
      (goto _label))))

(event `self.K2_OnEndAbility`
  (params (bWasCancelled :type Boolean)))